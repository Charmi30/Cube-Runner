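; BP_Cube is a physics-driven cube that moves forward on its own and is steered left and right by player input.
; A looping timer started on BeginPlay applies forward velocity-change impulses along X, while the Move left/right axis applies scaled impulses along Y.
; A Canmove flag gates both, and hitting an actor tagged "obstacle" clears it, ending further propulsion and steering.
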(event OnComponentHit(Cube)
  (params (HitComponent :type Primitive%20Component%20Object%20Reference) (OtherActor :type Actor%20Object%20Reference) (OtherComp :type Primitive%20Component%20Object%20Reference) (NormalImpulse :type Vector :default "0, 0, 0") (Hit :type Hit%20Result%20Structure%20%28by%20ref%29))
  (if (Actor|ActorHasTag OtherActor "obstacle")
    (Variables|Default|Setcanmove? false)))

(event Custom|MoveCube
  (if (Variables|Default|Getcanmove?)
    (Physics|AddImpulse (Variables|Default|GetCube) (Math|Vector|MakeVector (Variables|Default|GetForwardForce) 0.0 0.0) "None" true)))

(event EventBeginPlay
  (Utilities|Time|SetTimerbyEvent (delegate Custom|MoveCube) 0.1 true))

(event Input|AxisEvents|InputAxisMoveleft/right
  (params (AxisValue :type Float%20%28single-precision%29))
  (if (Variables|Default|Getcanmove?)
    (Physics|AddImpulse (Variables|Default|GetCube) (Math|Vector|MakeVector 0.0 (* AxisValue (Variables|Default|GetMoveright/leftforce)) 0.0) "None" true)))

(fn ConstructionScript)